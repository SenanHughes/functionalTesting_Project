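; Test floor manager for what appears to be a lane-based endless runner, spawning three starting floor segments and three lane positions.
; Each spawnNewFloor call adds a segment ahead and rolls floors through FloorsAfter and FloorsBefore, destroying the oldest once three lie behind.
; It also places one reused coin in a random lane ahead of the player.
; Hurdle spawning is an empty stub, and the random material colour helper is never called here.
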(event `self.ReceiveBeginPlay`
  (for _index (range 3)
    (bind _returnvalue (`|SpawnActorFromClass` "/Game/Blueprints/BP_Floor.BP_Floor_C" (`KismetMathLibrary.MakeTransform` (`KismetMathLibrary.MakeVector` (`KismetMathLibrary.Conv_IntToDouble` (* _index 1200)))) "Undefined" "MultiplyWithRoot" null null))
    (`KismetArrayLibrary.Array_Add` (`self.floorsAfter`) _returnvalue)
    (`KismetArrayLibrary.Array_Add` (`self.horizPosArray`) (`KismetMathLibrary.Conv_IntToDouble` (+ -200 (* 200 _index))))
    (`|GenericCreateObject` "/Game/Blueprints/WBP_gameOverlay.WBP_gameOverlay_C")))

(event `spawnNewFloor`
  (bind _returnvalue (`|SpawnActorFromClass` "/Game/Blueprints/BP_Floor.BP_Floor_C" (`KismetMathLibrary.Conv_VectorToTransform` (+ (`self.K2_GetActorLocation` (`|GetArrayItem` (`self.floorsAfter`))) (`self.newFloorLocation`))) "Undefined" "MultiplyWithRoot" null null))
  (set `self.newestFloor` _returnvalue)
  (`self.spawnCoin`)
  (`self.floorManagement`))

(event `floorManagement`
  (if (< (`KismetArrayLibrary.Array_Length` (`self.floorsBefore`)) 3)
    (`KismetArrayLibrary.Array_Add` (`self.floorsBefore`) (`|GetArrayItem` (`self.floorsAfter`)))
    (`self.updateFloorsArrays` (`self.floorsAfter`) 0 (`self.newestFloor`))
    (else
      (`self.K2_DestroyActor` (`|GetArrayItem` (`self.floorsBefore`)))
      (`self.updateFloorsArrays` (`self.floorsBefore`) 0 (`|GetArrayItem` (`self.floorsAfter`)))
      (`self.updateFloorsArrays` (`self.floorsAfter`) 0 (`self.newestFloor`)))))

(event `spawnHurdle`)

(event `spawnCoin`
  (bind _firstpersonreference (`self.firstPersonReference`))
  (bind _outitem (`KismetArrayLibrary.Array_Random` (`self.horizPosArray`)))
  (bind _returnvalue (`GameplayStatics.GetActorOfClass` "/Game/FirstPerson/Blueprints/BP_FirstPersonCharacter.BP_FirstPersonCharacter_C"))
  (set `self.firstPersonReference` _returnvalue)
  (if (`self.isCoinSpawned`)
    (bind _spawnxlocation (`self.randomTransformLocation` _firstpersonreference 200.0 600.0))
    (`self.K2_SetActorLocation` (`self.coinReference`) (`KismetMathLibrary.MakeVector` _spawnxlocation _outitem) false false)
    (else
      (bind _spawnxlocation_2 (`self.randomTransformLocation` _firstpersonreference 200.0 600.0))
      (bind _returnvalue_2 (`|SpawnActorFromClass` "/Game/Tests/BetaTests/BP_FSTCoin.BP_FSTCoin_C" (`KismetMathLibrary.MakeTransform` (`KismetMathLibrary.MakeVector` _spawnxlocation_2 _outitem)) "Undefined" "MultiplyWithRoot" null null))
      (set `self.coinReference` _returnvalue_2)
      (set `self.isCoinSpawned` true))))

(fn `dynamicMaterialColours`
  (params (self2 :type "/Game/Blueprints/BP_Floor Object Reference"))
  (bind _returnvalue (`PrimitiveComponent.CreateDynamicMaterialInstance` (`/Game/Blueprints/BP_Floor.StaticMesh` self2) 0 "/Game/Materials/dynamicColours_M.dynamicColours_M" "None"))
  (`MaterialInstanceDynamic.SetVectorParameterValue` _returnvalue "myColour" (`KismetMathLibrary.MakeColor` (`KismetMathLibrary.RandomFloatInRange` 0.0 1.0) (`KismetMathLibrary.RandomFloatInRange` 0.0 1.0) (`KismetMathLibrary.RandomFloatInRange` 0.0 1.0))))

(fn `randomTransformLocation`
  (params (actorReference :type "Actor Object Reference") (minSpawnVariance :type "Float (double-precision)") (maxSpawnVariance :type "Float (double-precision)"))
  (returns (spawnXLocation :type "Float (double-precision)"))
  (bind _returnvalue_x (`KismetMathLibrary.BreakVector` (`self.K2_GetActorLocation` actorReference)))
  (return (+ _returnvalue_x (`KismetMathLibrary.RandomFloatInRange` minSpawnVariance maxSpawnVariance))))

(fn `updateFloorsArrays`
  (params (updatingFloorArray :type "Array of /Game/Blueprints/BP_Floor Object Reference (by ref)") (floorIndexToRemove :type Integer) (newFloor :type "/Game/Blueprints/BP_Floor Object Reference (by ref)"))
  (`KismetArrayLibrary.Array_Remove` updatingFloorArray floorIndexToRemove)
  (`KismetArrayLibrary.Array_Add` updatingFloorArray newFloor))

(fn `UserConstructionScript`)