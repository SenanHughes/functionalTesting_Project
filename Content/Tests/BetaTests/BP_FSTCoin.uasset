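; BP_FSTCoin is a coin pickup that awards 200 points when the first-person character overlaps its box.
; It finds the game overlay widget by class, adds to its Score and calls IncreaseScore, so the score lives in the UI.
; It then destroys itself and clears IsCoinSpawned on the first BP_FSTfloorManagement actor found in the level.
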(event `self.Box.OnComponentBeginOverlap`
  (params (OverlappedComponent :type "PrimitiveComponent Object Reference") (OtherActor :type "Actor Object Reference") (OtherComp :type "PrimitiveComponent Object Reference") (OtherBodyIndex :type Integer) (bFromSweep :type Boolean) (SweepResult :type "HitResult Structure (by ref)"))
  (cast `/Game/FirstPerson/Blueprints/BP_FirstPersonCharacter` OtherActor)
  (bind _foundwidgets (`WidgetBlueprintLibrary.GetAllWidgetsOfClass` "/Game/Blueprints/WBP_gameOverlay.WBP_gameOverlay_C"))
  (bind _output (`|GetArrayItem` _foundwidgets))
  (set `/Game/Blueprints/WBP_gameOverlay.score` (+ (`/Game/Blueprints/WBP_gameOverlay.score` _output) 200) _output)
  (`/Game/Blueprints/WBP_gameOverlay.increaseScore` _output)
  (`self.K2_DestroyActor`)
  (bind _outactors (`GameplayStatics.GetAllActorsOfClass` "/Game/Tests/BetaTests/BP_FSTfloorManagement.BP_FSTfloorManagement_C"))
  (set `/Game/Tests/BetaTests/BP_FSTfloorManagement.isCoinSpawned` false (`|GetArrayItem` _outactors)))

(fn `UserConstructionScript`)