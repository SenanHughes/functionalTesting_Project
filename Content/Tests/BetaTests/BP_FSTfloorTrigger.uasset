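; Trigger actor for a floor-spawning test that advances ahead of the player and requests a new floor each time it is reached.
; When BP_FirstPersonCharacter overlaps EndpointTrigger, the actor jumps 1200 units along X to a random Y from BP_FSTfloorManagement's HorizPosArray.
; It then broadcasts its new location through TriggerLocation and calls SpawnNewFloor on the manager tagged managementTag.
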(event `self.endpointTrigger.OnComponentBeginOverlap`
  (params (OverlappedComponent :type "PrimitiveComponent Object Reference") (OtherActor :type "Actor Object Reference") (OtherComp :type "PrimitiveComponent Object Reference") (OtherBodyIndex :type Integer) (bFromSweep :type Boolean) (SweepResult :type "HitResult Structure (by ref)"))
  (bind _returnvalue (`self.K2_GetActorLocation`))
  (bind (_returnvalue_x _returnvalue_y _returnvalue_z) (`KismetMathLibrary.BreakVector` (+ _returnvalue (1200.0 0.0 0.0))))
  (cast `/Game/FirstPerson/Blueprints/BP_FirstPersonCharacter` OtherActor)
  (bind _outactors (`GameplayStatics.GetAllActorsOfClass` "/Game/Tests/BetaTests/BP_FSTfloorManagement.BP_FSTfloorManagement_C"))
  (`self.K2_SetActorLocation` (`KismetMathLibrary.MakeVector` _returnvalue_x (`KismetArrayLibrary.Array_Random` (`/Game/Tests/BetaTests/BP_FSTfloorManagement.horizPosArray` (`|GetArrayItem` _outactors))) _returnvalue_z))
  (`self.triggerLocation` _returnvalue)
  (bind _outactors_2 (`GameplayStatics.GetAllActorsOfClassWithTag` "/Game/Tests/BetaTests/BP_FSTfloorManagement.BP_FSTfloorManagement_C" "managementTag"))
  (`/Game/Tests/BetaTests/BP_FSTfloorManagement.spawnNewFloor` (`|GetArrayItem` _outactors_2)))

(fn `UserConstructionScript`)