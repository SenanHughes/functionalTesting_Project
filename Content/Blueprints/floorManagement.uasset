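; Floor manager Blueprint that builds a continuous track of BP_Floor segments along the X axis.
; BeginPlay lays out three evenly spaced floors in FloorsAfter.
; Each spawnNewFloor call adds a floor beyond the last, then floorManagement shifts the oldest ahead floor into FloorsBefore.
; Once FloorsBefore holds three, its oldest is destroyed, keeping a sliding window of segments by spawning and destroying rather than pooling.
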(event `self.ReceiveBeginPlay`
  (for _index (range 3)
    (bind _returnvalue (`|SpawnActorFromClass` "/Game/Blueprints/BP_Floor.BP_Floor_C" (`KismetMathLibrary.MakeTransform` (`KismetMathLibrary.MakeVector` (`KismetMathLibrary.Conv_IntToDouble` (* _index 1200)))) "Undefined" "MultiplyWithRoot" null null))
    (`KismetArrayLibrary.Array_Add` (`self.floorsAfter`) _returnvalue)))

(event `spawnNewFloor`
  (bind _returnvalue (`|SpawnActorFromClass` "/Game/Blueprints/BP_Floor.BP_Floor_C" (`KismetMathLibrary.Conv_VectorToTransform` (+ (`self.K2_GetActorLocation` (`|GetArrayItem` (`self.floorsAfter`))) (3600.0 0.0 0.0))) "Undefined" "MultiplyWithRoot" null null))
  (set `self.newestFloor` _returnvalue)
  (`self.floorManagement`))

(event `floorManagement`
  (bind _floorsafter (`self.floorsAfter`))
  (bind _floorsafter_2 (`self.floorsAfter`))
  (if (< (`KismetArrayLibrary.Array_Length` (`self.floorsBefore`)) 3)
    (`KismetArrayLibrary.Array_Add` (`self.floorsBefore`) (`|GetArrayItem` (`self.floorsAfter`)))
    (`KismetArrayLibrary.Array_Remove` _floorsafter_2)
    (`KismetArrayLibrary.Array_Add` _floorsafter_2 (`self.newestFloor`))
    (else
      (`self.K2_DestroyActor` (`|GetArrayItem` (`self.floorsBefore`)))
      (`KismetArrayLibrary.Array_Remove` (`self.floorsBefore`))
      (`KismetArrayLibrary.Array_Add` (`self.floorsBefore`) (`|GetArrayItem` (`self.floorsAfter`)))
      (`KismetArrayLibrary.Array_Remove` _floorsafter)
      (`KismetArrayLibrary.Array_Add` _floorsafter (`self.newestFloor`)))))

(fn `initialiseFloors`)

(fn `UserConstructionScript`)